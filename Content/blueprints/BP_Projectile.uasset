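; BP_Projectile is a projectile actor that explodes on a short fixed timer after it spawns.
; BeginPlay waits, calls Explode, then destroys the actor; the graph has no impact or collision trigger.
; Explode spawns a particle effect, applies radial damage credited to the first player controller, and draws a debug sphere at the blast location.
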(event `self.ReceiveBeginPlay`
  (`KismetSystemLibrary.Delay` 1.0)
  (`self.Explode`)
  (`self.K2_DestroyActor` self))

(event `Explode`
  (bind _returnvalue (`self.K2_GetActorLocation`))
  (`GameplayStatics.SpawnEmitterAtLocation` "/Game/WeaponEffects/Explosion/P_Explosion.P_Explosion" _returnvalue (`self.K2_GetActorRotation`))
  (`GameplayStatics.ApplyRadialDamage` :`BaseDamage` 15.0 :`Origin` _returnvalue :`DamageRadius` 200.0 :`DamageCauser` self :`InstigatedByController` (`GameplayStatics.GetPlayerController` 0))
  (`KismetSystemLibrary.DrawDebugSphere` _returnvalue 20.0 12 (struct :`R` 1.0 :`G` 0.985008 :`B` 0.172875 :`A` 1.0) 1.0 2.0))

(fn `UserConstructionScript`)